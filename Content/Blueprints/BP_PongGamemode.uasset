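; Pong game mode that keeps score for player-versus-AI and two-player matches and resets the ball after each point.
; Separate events for each of the four point outcomes increment the matching score and play one of two 8-bit beeps.
; Each event then destroys the BP_Ball found in the level and, after a short delay, spawns a new one at a fixed central location.
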(event `self.ReceiveBeginPlay`)

(event `PlayerWin`
  (`/Engine/EditorBlueprintResources/StandardMacros.IncrementInt` (`self.PlayerScore`)
    (:`  `
      (`GameplayStatics.SpawnSound2D` "/Game/misc/SFX/ping_pong_8bit_beeep.ping_pong_8bit_beeep" 1.0 1.0 0.0 null)
      (bind _returnvalue (`GameplayStatics.GetActorOfClass` "/Game/Blueprints/BP_Ball.BP_Ball_C"))
      (`self.K2_DestroyActor` _returnvalue)
      (`KismetSystemLibrary.Delay` 1.0)
      (`|SpawnActorFromClass` "/Game/Blueprints/BP_Ball.BP_Ball_C" (`KismetMathLibrary.MakeTransform` (0.0 0.0 30.0)) "Undefined" "MultiplyWithRoot" null null))))

(event `PlayerLose`
  (`/Engine/EditorBlueprintResources/StandardMacros.IncrementInt` (`self.AIScore`)
    (:`  `
      (`GameplayStatics.SpawnSound2D` "/Game/misc/SFX/ping_pong_8bit_peeeeeep.ping_pong_8bit_peeeeeep" 1.0 1.0 0.0 null)
      (bind _returnvalue (`GameplayStatics.GetActorOfClass` "/Game/Blueprints/BP_Ball.BP_Ball_C"))
      (`self.K2_DestroyActor` _returnvalue)
      (`KismetSystemLibrary.Delay` 1.0)
      (`|SpawnActorFromClass` "/Game/Blueprints/BP_Ball.BP_Ball_C" (`KismetMathLibrary.MakeTransform` (0.0 0.0 30.0)) "Undefined" "MultiplyWithRoot" null null))))

(event `Player1Win`
  (`/Engine/EditorBlueprintResources/StandardMacros.IncrementInt` (`self.Player1Score`)
    (:`  `
      (`GameplayStatics.SpawnSound2D` "/Game/misc/SFX/ping_pong_8bit_beeep.ping_pong_8bit_beeep" 1.0 1.0 0.0 null)
      (bind _returnvalue (`GameplayStatics.GetActorOfClass` "/Game/Blueprints/BP_Ball.BP_Ball_C"))
      (`self.K2_DestroyActor` _returnvalue)
      (`KismetSystemLibrary.Delay` 1.0)
      (`|SpawnActorFromClass` "/Game/Blueprints/BP_Ball.BP_Ball_C" (`KismetMathLibrary.MakeTransform` (0.0 0.0 30.0)) "Undefined" "MultiplyWithRoot" null null))))

(event `Player2Win`
  (`/Engine/EditorBlueprintResources/StandardMacros.IncrementInt` (`self.Player2Score`)
    (:`  `
      (`GameplayStatics.SpawnSound2D` "/Game/misc/SFX/ping_pong_8bit_peeeeeep.ping_pong_8bit_peeeeeep" 1.0 1.0 0.0 null)
      (bind _returnvalue (`GameplayStatics.GetActorOfClass` "/Game/Blueprints/BP_Ball.BP_Ball_C"))
      (`self.K2_DestroyActor` _returnvalue)
      (`KismetSystemLibrary.Delay` 1.0)
      (`|SpawnActorFromClass` "/Game/Blueprints/BP_Ball.BP_Ball_C" (`KismetMathLibrary.MakeTransform` (0.0 0.0 30.0)) "Undefined" "MultiplyWithRoot" null null))))

(fn `UserConstructionScript`)