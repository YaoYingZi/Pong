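; BP_Ball is a ball actor that plays an 8-bit ping-pong plop sound whenever its Sphere component registers a hit.
; The Construction Script gives the Sphere a random world yaw across the full circle, adding an offset when the angle falls near plus or minus 90 degrees to keep it out of those bands.
; No movement logic appears in its graphs.
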(event `self.Sphere.OnComponentHit`
  (params (HitComponent :type "PrimitiveComponent Object Reference") (OtherActor :type "Actor Object Reference") (OtherComp :type "PrimitiveComponent Object Reference") (NormalImpulse :type "Vector Structure") (Hit :type "HitResult Structure (by ref)"))
  (`GameplayStatics.PlaySound2D` "/Game/misc/SFX/ping_pong_8bit_plop.ping_pong_8bit_plop" 1.0 1.0 0.0 null null))

(fn `UserConstructionScript`
  (bind _returnvalue (`KismetMathLibrary.Abs` (`self.RSpeed`)))
  (set `self.RSpeed` (`KismetMathLibrary.RandomFloatInRange` -180.0 180.0))
  (if (and (> _returnvalue 80.0) (< _returnvalue 100.0))
    (bind _output_get (set `self.RSpeed` (+ (`self.RSpeed`) 30.0)))
    (`SceneComponent.K2_SetWorldRotation` (`self.Sphere`) (`KismetMathLibrary.MakeRotator` 0.0 0.0 _output_get) false false)
    (else
      (`SceneComponent.K2_SetWorldRotation` (`self.Sphere`) (`KismetMathLibrary.MakeRotator` 0.0 0.0 (`self.RSpeed`)) false false))))