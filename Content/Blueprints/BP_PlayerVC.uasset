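; BP_PlayerVC is the player-controlled paddle for a Pong game, using Enhanced Input.
; When the controller changes, it adds the IMC_Pong mapping context to the player controller's input subsystem.
; The BasicMove action offsets the Cube along world Y by the input value times Speed, clamped to fixed limits.
; Movement sets world location directly, without sweep or delta-time scaling.
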(event `self.ReceiveControllerChanged`
  (params (OldController :type "Controller Object Reference") (NewController :type "Controller Object Reference"))
  (bind `_as玩家控制器` (cast `PlayerController` NewController))
  (`EnhancedInputSubsystemInterface.AddMappingContext` (pcsubsystem `EnhancedInputLocalPlayerSubsystem` `_as玩家控制器`) "/Game/misc/IMC_Pong.IMC_Pong" 0 (struct)))

(event `self.ReceiveBeginPlay`)

(event `EnhancedInput|/Game/misc/BasicMove`
  (params (ActionValue :type "Float (double-precision)") (ElapsedSeconds :type "Float (double-precision)") (TriggeredSeconds :type "Float (double-precision)") (InputAction :type "InputAction Object Reference" :default "/Game/misc/BasicMove.BasicMove"))
  (bind (_returnvalue_x _returnvalue_y _returnvalue_z) (`KismetMathLibrary.BreakVector` (`SceneComponent.K2_GetComponentLocation` (`self.Cube`))))
  (:`Triggered`
    (`SceneComponent.K2_SetWorldLocation` (`self.Cube`) (`KismetMathLibrary.MakeVector` _returnvalue_x (`KismetMathLibrary.FClamp` (+ (* ActionValue (`self.Speed`)) _returnvalue_y) -400.0 390.0) _returnvalue_z) false false)))

(fn `UserConstructionScript`)