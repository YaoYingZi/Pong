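; AI-controlled actor that follows the ball sideways, apparently an opponent paddle in a Pong-style game.
; Every Tick it searches for all BP_Ball actors and takes the first one, staying put if none exist.
; It interpolates toward that ball's Y position, clamped to fixed bounds, at InterpSpeed without sweep, keeping its own X and Z.
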(event `self.ReceiveTick`
  (params (DeltaSeconds :type "Float (single-precision)"))
  (bind (_returnvalue_x _returnvalue_y _returnvalue_z) (`KismetMathLibrary.BreakVector` (`self.K2_GetActorLocation`)))
  (bind _outactors (`GameplayStatics.GetAllActorsOfClass` "/Game/Blueprints/BP_Ball.BP_Ball_C"))
  (if (> (`KismetArrayLibrary.Array_Length` _outactors) 0)
    (bind (_returnvalue_x_2 _returnvalue_y_2) (`KismetMathLibrary.BreakVector` (`self.K2_GetActorLocation` (`|GetArrayItem` _outactors))))
    (`self.K2_SetActorLocation` (`KismetMathLibrary.VInterpTo` (`KismetMathLibrary.MakeVector` _returnvalue_x _returnvalue_y _returnvalue_z) (`KismetMathLibrary.MakeVector` _returnvalue_x (`KismetMathLibrary.FClamp` _returnvalue_y_2 -400.0 390.0) _returnvalue_z) DeltaSeconds (`self.Interp Speed`)))))

(fn `UserConstructionScript`)